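; BP_PlayerPawn is the player pawn Blueprint that sets up the player's crosshair and ammo count HUD.
; On BeginPlay it creates the WBP_Crosshair and WBP_AmmoCount widgets, adds both to the viewport and keeps a reference to the ammo widget.
; Every Tick it pushes the current weapon's ammo count into that widget by polling rather than using events.
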(event `self.ReceiveBeginPlay`
  (bind _returnvalue (`|CreateWidget` "/Game/UI/WBP_Crosshair.WBP_Crosshair_C"))
  (`UserWidget.AddToViewport` _returnvalue 0)
  (bind _returnvalue_2 (`|CreateWidget` "/Game/UI/WBP_AmmoCount.WBP_AmmoCount_C"))
  (bind _aswbp_ammo_count (cast `/Game/UI/WBP_AmmoCount` _returnvalue_2))
  (set `self.AmmoCountUI` _aswbp_ammo_count)
  (`UserWidget.AddToViewport` _returnvalue_2 0))

(event `self.ReceiveTick`
  (params (DeltaSeconds :type "Float (single-precision)"))
  (bind _aswbp_ammo_count (cast `/Game/UI/WBP_AmmoCount` (`self.AmmoCountUI`)))
  (set `/Game/UI/WBP_AmmoCount.UICurrentAmmoCount` (`SWeapon.CurrentAmmoCount` (`self.CurrentWeapon`)) _aswbp_ammo_count))

(fn `UserConstructionScript`)